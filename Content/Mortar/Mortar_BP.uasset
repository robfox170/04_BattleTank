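; Mortar actor Blueprint that reuses the tank aiming component and carries a health bar widget.
; On BeginPlay it initializes TankAiming with its Barrel and Dome, the dome serving as the turret.
; It then casts the HealthBar component's widget to HealthBar_BP and passes itself in as the tank reference, skipping this if the cast fails.
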(event EventBeginPlay
  (Class|TankAimingComponent|Initialize (Variables|Default|GetTankAiming) (Variables|Default|GetBarrel) (Variables|Default|GetDome))
  (CallFunction|InitializeHealthBarWidget))

(fn ConstructionScript)

(fn InitializeHealthBarWidget
  (bind _ashealth_bar_bp (Utilities|Casting|CastToHealthBar_BP (UserInterface|GetUserWidgetObject (Variables|Default|GetHealthBar))))
  (Variables|/Game/UI/HealthBar_BP.HealthBar_BP_C|SetBP%20Tank%20Reference _ashealth_bar_bp self))