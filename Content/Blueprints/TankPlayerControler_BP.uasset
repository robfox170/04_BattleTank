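; Player controller Blueprint for a tank game that manages the player's HUD and death flow.
; When the aiming component is found, it creates the PlayerUI_BP widget, adds it to the viewport and passes it the aiming component reference.
; On BeginPlay it binds to the controlled Tank's OnDeath delegate, which notifies the UI of the death, then opens MainMenu after a delay.
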(event Custom|OnDeath_Event_0
  ;[1 1 1] Binding to OnDeath delegate (declared in Tank.h) to access PlayerUI_BP method OnPlayerTankDeath (hides aimpoint and rounds left, and displays "You're Dead")
  (bind _foundwidgets (Widget|GetAllWidgetsOfClass "/Game/UI/PlayerUI_BP.PlayerUI_BP_C" true))
  (Default|OnPlayerTankDeath (Utilities|Array|Get(acopy) _foundwidgets))
  (Utilities|FlowControl|Delay 6e+01) ; Optionally, could go to main menu automatically after a while
  (Game|OpenLevel(byName) "MainMenu"))

(event EventFoundAimingComponent
  (params (AimCompRef :type Tank%20Aiming%20Component%20Object%20Reference))
  ;[1 1 1] Adding an aimpoint widget to the viewport
  (bind _returnvalue (UserInterface|CreateWidget "/Game/UI/PlayerUI_BP.PlayerUI_BP_C"))
  (UserInterface|Viewport|AddtoViewport _returnvalue 0)
  (Variables|/Game/UI/PlayerUI_BP.PlayerUI_BP_C|SetBP%20Aiming%20Comp%20Reference _returnvalue AimCompRef))

(event EventBeginPlay
  ;[1 1 1] Binding to OnDeath delegate (declared in Tank.h) to access PlayerUI_BP method OnPlayerTankDeath (hides aimpoint and rounds left, and displays "You're Dead")
  (bind _astank (Utilities|Casting|CastToTank (Pawn|GetControlledPawn)))
  (EventDispatchers|AssignOnDeath _astank (delegate Custom|OnDeath_Event_0)))

(fn ConstructionScript)